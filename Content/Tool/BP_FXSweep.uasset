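; BP_FXSweep is a generated dynamic mesh tool that builds FX meshes by sweeping a spline-drawn profile along a spline path.
; Rebuild flattens SplineBase into a 2D polygon and sweeps it uncapped along SplinePath with start/end scaling, then recomputes normals and optionally rotates UVs.
; The construction script shifts both splines by the Offset location.
; BakeMesh saves the result as a uniquely named SM_FX_ static mesh asset, carrying over materials.
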(event Custom|Bake%20Mesh
  ;[1 1 1] Bake to Static Mesh
  (bind _returnvalue (DynamicMeshComponent|GetDynamicMesh (Variables|DynamicMeshActor|GetDynamicMeshComponent)))
  (bind _uniqueassetpathandname (Class|GeometryScriptLibraryCreateNewAssetFunctions|CreateUniqueNewAssetPathName :AssetFolderPath (Variables|Default|GetAsset%20Path) :BaseAssetName "SM_FX_" :Debug 0)
    (:Failure
      (Development|PrintString "Failed !"))
    (:Success
      (bind _returnvalue_2 (GeometryScript|AssetManagement|CreateNewStaticMeshAssetfromMesh _returnvalue _uniqueassetpathandname (Utilities|Struct|MakeGeometryScriptCreateNewStaticMeshAssetOptions true true false 0.0 true "CTF_UseDefault") 0)
        (:Failure
          (Development|PrintString "Failed to Create Asset"))
        (:Success
          (for (_array_element _array_index) (Rendering|Material|GetMaterials (Variables|DynamicMeshActor|GetDynamicMeshComponent))
            (Rendering|Material|SetMaterial _returnvalue_2 _array_index _array_element)))))))

(event Events|EventOnRebuildGeneratedMesh
  (params (TargetMesh :type Dynamic%20Mesh%20Object%20Reference))
  ;[1 1 1] Generate Mesh
  (Utilities|Array|Clear (Variables|Default|GetPoints))
  (Utilities|FlowControl|Sequence
    (:then_0
      (Variables|Default|SetOut%20Points (.OutPoints (Class|SplineComponent|ConvertSplinetoPolyLine (Variables|Default|GetSpline_Path) "Local" 0.5)))
      (for _array_element (.OutPoints (Class|SplineComponent|ConvertSplinetoPolyLine (Variables|Default|GetSpline_Base) "Local" 0.5))
        (Utilities|Array|Add (Variables|Default|GetPoints) (Math|Vector2D|MakeVector2D (* (.z _array_element) -1.0) (.y _array_element)))))
    (:then_1
      (bind _returnvalue (Class|GeometryScriptLibraryMeshPrimitiveFunctions|AppendSimpleSweptPolygon :TargetMesh TargetMesh :Transform (Variables|Default|GetOffset) :PolygonVertices (Variables|Default|GetPoints) :SweepPath (Variables|Default|GetOut%20Points) :bCapped false :StartScale (Variables|Default|GetStart%20Scale) :EndScale (Variables|Default|GetEnd%20Scale) :Debug 0))
      (bind _returnvalue_2 (GeometryScript|Normals|RecomputeNormals :TargetMesh _returnvalue :Debug 0))
      (if (Variables|Default|GetRotate)
        (Class|GeometryScriptLibraryMeshUVFunctions|RotateMeshUVs _returnvalue_2 0 9e+01 "(X=0.000000,Y=0.000000)" 0)))))

(fn ConstructionScript
  (bind _offset (Variables|Default|GetOffset))
  (Transformation|AddLocalOffset (Variables|Default|GetSpline_Path) (.location _offset) false false)
  (Transformation|AddLocalOffset (Variables|Default|GetSpline_Base) (.location _offset) false false))