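; Editor tool actor that procedurally generates FX meshes from a spline profile using Geometry Script and bakes them to static mesh assets.
; On rebuild, the spline's XZ polyline is revolved, twisted, repeated around yaw, then given recomputed normals and optionally rotated UVs.
; BakeMesh saves the dynamic mesh as a uniquely named SM_FX_ asset and copies over the component's materials.
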(event Custom|Bake%20Mesh
  ;[1 1 1] Bake to Static Mesh
  (bind _returnvalue (DynamicMeshComponent|GetDynamicMesh (Variables|DynamicMeshActor|GetDynamicMeshComponent)))
  (bind _uniqueassetpathandname (Class|GeometryScriptLibraryCreateNewAssetFunctions|CreateUniqueNewAssetPathName :AssetFolderPath (Variables|Default|GetAsset%20Path) :BaseAssetName "SM_FX_" :Debug 0)
    (:Failure
      (Development|PrintString "Failed !"))
    (:Success
      (bind _returnvalue_2 (GeometryScript|AssetManagement|CreateNewStaticMeshAssetfromMesh _returnvalue _uniqueassetpathandname (Utilities|Struct|MakeGeometryScriptCreateNewStaticMeshAssetOptions true true false 0.0 true "CTF_UseDefault") 0)
        (:Failure
          (Development|PrintString "Failed to Create Asset"))
        (:Success
          (for (_array_element _array_index) (Rendering|Material|GetMaterials (Variables|DynamicMeshActor|GetDynamicMeshComponent))
            (Rendering|Material|SetMaterial _returnvalue_2 _array_index _array_element)))))))

(event Events|EventOnRebuildGeneratedMesh
  (params (TargetMesh :type Dynamic%20Mesh%20Object%20Reference))
  (bind _repeat_count (Variables|Default|GetRepeat%20Count))
  ;[1 1 1] Generate Mesh
  (Utilities|Array|Clear (Variables|Default|GetPoints))
  (Utilities|FlowControl|Sequence
    (:then_0
      (for _array_element (.OutPoints (Class|SplineComponent|ConvertSplinetoPolyLine (Variables|Default|GetSpline) "Local" (Variables|Default|GetSmoothness)))
        (Utilities|Array|Add (Variables|Default|GetPoints) (Math|Vector2D|MakeVector2D (.x _array_element) (.z _array_element)))))
    (:then_1
      (bind _returnvalue (DynamicMeshActor|AllocateComputeMesh))
      (bind _returnvalue_2 (Class|GeometryScriptLibraryMeshPrimitiveFunctions|AppendRevolvePath :TargetMesh _returnvalue :PrimitiveOptions (Utilities|Struct|MakeGeometryScriptPrimitiveOptions "PerFace" (Variables|Default|GetFlip%20Orientation) "Uniform") :PathVertices (Variables|Default|GetPoints) :RevolveOptions (Utilities|Struct|MakeGeometryScriptRevolveOptions (Variables|Default|GetDegrees) (Variables|Default|GetDegree%20Offset) true) :Steps (Variables|Default|GetSteps) :bCapped false :Debug 0))
      (bind _returnvalue_3 (Class|GeometryScriptLibraryMeshDeformFunctions|ApplyTwistWarptoMesh :TargetMesh _returnvalue_2 :TwistAngle (Variables|Default|GetTwist%20Angle) :TwistExtent (Spline|GetSplineLength (Variables|Default|GetSpline)) :Debug 0))
      (Variables|Default|SetTarget%20Mesh _returnvalue_3))
    (:then_2
      (bind _returnvalue_4 (Class|GeometryScriptLibraryMeshBasicEditFunctions|AppendMeshRepeated TargetMesh (Variables|Default|GetTarget%20Mesh) (Math|Transform|MakeTransform "0, 0, 0" (Math|Rotator|MakeRotator 0.0 0.0 (Math|Conversions|ToFloat(Integer) (/ 360 _repeat_count))) "1.000000,1.000000,1.000000") _repeat_count true true 0))
      (bind _returnvalue_5 (GeometryScript|Normals|RecomputeNormals :TargetMesh _returnvalue_4 :Debug 0))
      (if (Variables|Default|GetRotate)
        (Class|GeometryScriptLibraryMeshUVFunctions|RotateMeshUVs _returnvalue_5 0 9e+01 "(X=0.000000,Y=0.000000)" 0)))))

(fn ConstructionScript)